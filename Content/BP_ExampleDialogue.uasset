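; Example dialogue participant Blueprint that demonstrates and exercises a dialogue plugin's Blueprint API.
; Its participant functions read and write bool, int, float and name values in DialogueData, with bools stored as a set of true names; condition, event and icon handlers are stubs.
; An ALL_FUNCTIONS graph collects unwired plugin nodes.
; Disconnected construction-script code tests Select and Switch nodes on variable names and can start a dialogue.
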(fn `CheckCondition`
  (params (Context :type "DlgContext Object Reference") (ConditionName :type Name))
  (returns (ReturnValue :type Boolean))
  (return false))

(fn `GetBoolValue`
  (params (ValueName :type Name))
  (returns (ReturnValue :type Boolean))
  (return (`BlueprintSetLibrary.Set_Contains` (`.TrueBools_14_7A9E751B448C8D29C7289BA1CA5763E0` (break `/DlgSystem/Struct_ExampleDialogueData` (`self.DialogueData`))) ValueName)))

(fn `GetFloatValue`
  (params (ValueName :type Name))
  (returns (ReturnValue :type "Float (double-precision)"))
  (return (`BlueprintMapLibrary.Map_Find` (`.Floats_8_1BEDFB974C56C4E6619D6185520AC0F5` (break `/DlgSystem/Struct_ExampleDialogueData` (`self.DialogueData`))) ValueName)))

(fn `GetIntValue`
  (params (ValueName :type Name))
  (returns (ReturnValue :type Integer))
  (return (`BlueprintMapLibrary.Map_Find` (`.Integers_5_BDAD136B4844D6F79F342A955D057FD8` (break `/DlgSystem/Struct_ExampleDialogueData` (`self.DialogueData`))) ValueName)))

(fn `GetNameValue`
  (params (ValueName :type Name))
  (returns (ReturnValue :type Name))
  (return (`BlueprintMapLibrary.Map_Find` (`.Names_11_B12748B04CECF30187E8ACBECB4A55AC` (break `/DlgSystem/Struct_ExampleDialogueData` (`self.DialogueData`))) ValueName)))

(fn `GetParticipantDisplayName`
  (params (ActiveSpeaker :type Name))
  (returns (ReturnValue :type Text))
  (return (`KismetTextLibrary.Conv_NameToText` (`self.DialogueParticipantName`))))

(fn `GetParticipantGender`
  (returns (ReturnValue :type "ETextGender Enum"))
  (return "Masculine"))

(fn `GetParticipantIcon`
  (params (ActiveSpeaker :type Name) (ActiveSpeakerState :type Name))
  (returns (ReturnValue :type "Texture2D Object Reference"))
  (return null))

(fn `GetParticipantName`
  (returns (ReturnValue :type Name))
  (return (`self.DialogueParticipantName`)))

(fn `ModifyBoolValue`
  (params (ValueName :type Name) (bNewValue :type Boolean))
  (returns (ReturnValue :type Boolean))
  (bind (_integers _floats _names _truebools) (break `/DlgSystem/Struct_ExampleDialogueData` (`self.DialogueData`)))
  (if bNewValue
    (`BlueprintSetLibrary.Set_Add` _truebools ValueName)
    (else
      (`BlueprintSetLibrary.Set_Remove` _truebools ValueName)))
  (return false))

(fn `ModifyFloatValue`
  (params (ValueName :type Name) (bDelta :type Boolean) (Value :type "Float (double-precision)"))
  (returns (ReturnValue :type Boolean))
  (bind (_integers _floats) (break `/DlgSystem/Struct_ExampleDialogueData` (`self.DialogueData`)))
  (`BlueprintMapLibrary.Map_Add` _floats ValueName (select `bool` bDelta :`false` Value :`true` (+ Value (`BlueprintMapLibrary.Map_Find` _floats ValueName))))
  (return false))

(fn `ModifyIntValue`
  (params (ValueName :type Name) (bDelta :type Boolean) (Value :type Integer))
  (returns (ReturnValue :type Boolean))
  (bind _integers (break `/DlgSystem/Struct_ExampleDialogueData` (`self.DialogueData`)))
  (`BlueprintMapLibrary.Map_Add` _integers ValueName (select `bool` bDelta :`false` Value :`true` (+ Value (`BlueprintMapLibrary.Map_Find` _integers ValueName))))
  (return false))

(fn `ModifyNameValue`
  (params (ValueName :type Name) (NameValue :type Name))
  (returns (ReturnValue :type Boolean))
  (`BlueprintMapLibrary.Map_Add` (`.Names_11_B12748B04CECF30187E8ACBECB4A55AC` (break `/DlgSystem/Struct_ExampleDialogueData` (`self.DialogueData`))) ValueName NameValue)
  (return false))

(fn `OnDialogueEvent`
  (params (Context :type "DlgContext Object Reference") (EventName :type Name))
  (returns (ReturnValue :type Boolean))
  (`|SwitchDialogueCallbackEvent` EventName
    (:`Default`
      (return false))))

(fn `PrintStringWithNewLines`
  (params (ToPrint :type String) (NumNewLinesBefore :type Integer :default 1) (NumNewLinesAfter :type Integer :default 1))
  (for _ (range 1 (+ NumNewLinesBefore 1))
    (`KismetSystemLibrary.PrintString` ""))
  (`KismetSystemLibrary.PrintString` ToPrint)
  (for _ (range 1 (+ NumNewLinesAfter 1))
    (`KismetSystemLibrary.PrintString` "")))

(fn `UserConstructionScript`
  (locals (VariableName :type Name :default "EdgeVariable") (ParticipantData :type "Map of Name to DlgParticipantData Structure") (VariablesNum :type Integer) (IntNames :type "Array of Name") (FloatNames :type "Array of Name") (ParticipantName :type Name) (VariableNameDefault :type Name :default "AAAAAANoneDEFAULT") (ArrayIndex :type Integer :default 0) (ExecutionWireIndex :type Integer) (ExecutionWireIndexDefault :type Integer :default -1) (SelectIntReturnValue :type Integer) (SelectIntDefaultValue :type Integer :default -1) (bDefaultWasExecuted :type Boolean)))