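; Test Blueprint that acts as a dialogue participant to check the dialogue system's Select and Switch nodes for int variable names.
; The construction script gathers the participant's int and float names and appends a default name, but only the ints are tested.
; It compares each Select result and executed Switch pin with the name's index or default, printing results or errors.
; Participant interface functions are mostly stubs, and the StartDialogue chain never runs.
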(fn `CheckCondition`
  (params (DialogueName :type "Name (by ref)") (ConditionName :type "Name (by ref)"))
  (returns (ReturnValue :type Boolean))
  (return false))

(fn `GetBoolValue`
  (params (ValueName :type "Name (by ref)"))
  (returns (ReturnValue :type Boolean))
  (return false))

(fn `GetFloatValue`
  (params (ValueName :type "Name (by ref)"))
  (returns (ReturnValue :type "Float (double-precision)"))
  (return 0.0))

(fn `GetIntValue`
  (params (ValueName :type "Name (by ref)"))
  (returns (ReturnValue :type Integer))
  (return 0))

(fn `GetParticipantDisplayName`
  (returns (ReturnValue :type Text))
  (return (`KismetTextLibrary.Conv_NameToText` (`self.DlgOwner`))))

(fn `GetParticipantIcon`
  (returns (ReturnValue :type "Texture2D Object Reference"))
  (return null))

(fn `GetParticipantName`
  (returns (ReturnValue :type Name))
  (return (`self.DlgOwner`)))

(fn `ModifyBoolValue`
  (params (ValueName :type "Name (by ref)") (bNewValue :type Boolean))
  (returns (ReturnValue :type Boolean))
  (return false))

(fn `ModifyFloatValue`
  (params (ValueName :type "Name (by ref)") (bDelta :type Boolean) (Value :type "Float (double-precision)"))
  (returns (ReturnValue :type Boolean))
  (return false))

(fn `ModifyIntValue`
  (params (ValueName :type "Name (by ref)") (bDelta :type Boolean) (Value :type Integer))
  (returns (ReturnValue :type Boolean))
  (return false))

(fn `OnDialogueEvent`
  (params (DialogueName :type "Name (by ref)") (EventName :type "Name (by ref)"))
  (returns (ReturnValue :type Boolean))
  (return false))

(fn `PrintStringWIthNewLines`
  (params (ToPrint :type String) (NumNewLinesBefore :type Integer :default 1) (NumNewLinesAfter :type Integer :default 1))
  (for _ (range 1 (+ NumNewLinesBefore 1))
    (`KismetSystemLibrary.PrintString` ""))
  (`KismetSystemLibrary.PrintString` ToPrint)
  (for _ (range 1 (+ NumNewLinesAfter 1))
    (`KismetSystemLibrary.PrintString` "")))

(fn `UserConstructionScript`
  (locals (VariableName :type Name :default "EdgeVariable") (ParticipantData :type "Map of Name to DlgParticipantData Structure") (VariablesNum :type Integer) (IntNames :type "Array of Name") (FloatNames :type "Array of Name") (ParticipantName :type Name) (VariableNameDefault :type Name :default "AAAAAANoneDEFAULT") (ArrayIndex :type Integer :default 0) (ExecutionWireIndex :type Integer) (ExecutionWireIndexDefault :type Integer :default -1) (SelectIntReturnValue :type Integer) (SelectIntDefaultValue :type Integer :default -1) (bDefaultWasExecuted :type Boolean))
  (bind _returnvalue (`self.GetParticipantName`))
  (bind _arrayindex (`local.ArrayIndex`))
  (bind _returnvalue_2 (`KismetStringLibrary.Conv_IntToString` (`local.SelectIntReturnValue`)))
  (bind _returnvalue_3 (`KismetStringLibrary.Conv_NameToString` (`local.VariableName`)))
  ;[1 1 1] Get participant data from Dialogue
  (if (`DlgDialogue.IsParticipant` (`self.Dlg`) _returnvalue)
    (set `local.ParticipantName` _returnvalue)
    (`|ExecutionSequence`
      (:`then_0`
        ;[1 1 1] Int Variables
        (bind _output_get (set `local.IntNames` (`DlgManager.GetAllDialoguesIntNames` (`local.ParticipantName`))))
        (`KismetArrayLibrary.Array_Add` _output_get (`local.VariableNameDefault`)))
      (:`then_1`
        ;[1 1 1] Float Variables
        (bind _output_get_2 (set `local.FloatNames` (`DlgManager.GetAllDialoguesFloatNames` (`local.ParticipantName`))))
        (`KismetArrayLibrary.Array_Add` _output_get_2 (`local.VariableNameDefault`))
        (`|ExecutionSequence`
          (:`then_0`
            ;[1 1 1] Select
            (`self.PrintStringWIthNewLines` "=== SELECT ===")
            (for (_array_element _array_index) (`local.IntNames`)
              (bind _output_get_3 (set `local.VariableName` _array_element))
              (set `local.ArrayIndex` _array_index)
              (set `local.SelectIntReturnValue` (`|Select` _output_get_3 (`local.SelectIntDefaultValue`) _array_index _array_index _array_index _array_index))
              (if (!= (`local.VariableName`) (`local.VariableNameDefault`))
                ;[1 1 1] Normal Select
                (if (== (`local.SelectIntReturnValue`) _arrayindex)
                  (`KismetSystemLibrary.PrintString` (`KismetStringLibrary.Concat_StrStr` _returnvalue_3 " Select: " _returnvalue_2))
                  (else
                    (`KismetSystemLibrary.PrintString` (`KismetStringLibrary.Concat_StrStr` _returnvalue_3 " Select does does not MATCH return value. ERROR. " "ArrayIndex = " (`KismetStringLibrary.Conv_IntToString` _arrayindex) " ReturnValue = " _returnvalue_2))))
                (else
                  ;[1 1 1] Default select
                  (if (== (`local.SelectIntReturnValue`) (`local.SelectIntDefaultValue`))
                    (`KismetSystemLibrary.PrintString` "<Default Select>")
                    (else
                      (`KismetSystemLibrary.PrintString` (`KismetStringLibrary.Concat_StrStr` (`KismetStringLibrary.Conv_NameToString` (`local.VariableName`)) " Why isn't this the default return value? ERROR")))))))
            (`KismetSystemLibrary.PrintString` ""))
          (:`then_1`
            ;[1 1 1] Switch
            (`self.PrintStringWIthNewLines` "=== SWITCH ===")
            (for (_array_element_2 _array_index_2) (`local.IntNames`)
              (`|ExecutionSequence`
                (:`then_0`
                  (set `local.VariableName` _array_element_2)
                  (set `local.ArrayIndex` _array_index_2)
                  (set `local.ExecutionWireIndex` (`local.ExecutionWireIndexDefault`))
                  (`|SwitchDialogueCallbackIntValue` (`local.VariableName`)
                    (:`Default`
                      (set `local.bDefaultWasExecuted` true))
                    (:`Default`
                      (set `local.ExecutionWireIndex` 0))
                    (:`DefaultValue`
                      (set `local.ExecutionWireIndex` 1))
                    (:`EdgeVariable`
                      (set `local.ExecutionWireIndex` 2))
                    (:`NodeVariable`
                      (set `local.ExecutionWireIndex` 3))))
                (:`then_1`
                  (if (!= (`local.VariableName`) (`local.VariableNameDefault`))
                    ;[1 1 1] Normal Execution Option
                    (if (== (`local.ExecutionWireIndex`) (`local.ArrayIndex`))
                      (`KismetSystemLibrary.PrintString` (`KismetStringLibrary.Concat_StrStr` (`KismetStringLibrary.Conv_NameToString` (`local.VariableName`)) " Execution: " (`KismetStringLibrary.Conv_IntToString` (`local.ArrayIndex`))))
                      (else
                        (`KismetSystemLibrary.PrintString` (`KismetStringLibrary.Concat_StrStr` (`KismetStringLibrary.Conv_NameToString` (`local.VariableName`)) " Was executed for the wrong Execution Pin. ERROR. " "Execution Pin Index: " (`KismetStringLibrary.Conv_IntToString` (`local.ExecutionWireIndex`))))))
                    (else
                      ;[1 1 1] Default execution
                      (if (and (== (`local.ExecutionWireIndex`) (`local.ExecutionWireIndexDefault`)) (`local.bDefaultWasExecuted`))
                        (`KismetSystemLibrary.PrintString` "<Default Execution>")
                        (else
                          (`KismetSystemLibrary.PrintString` (`KismetStringLibrary.Concat_StrStr` (`KismetStringLibrary.Conv_NameToString` (`local.VariableName`)) " why isn't this the default execution value? Was the default pin even executed? ERROR. " "bDefaultWasExecuted = " (`KismetStringLibrary.Conv_BoolToString` (`local.bDefaultWasExecuted`)))))))))))
            (`KismetSystemLibrary.PrintString` "")))))
    (else
      (`KismetSystemLibrary.PrintString` "Failed to get Participant data for curent participant"))))